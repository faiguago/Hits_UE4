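; BP_Hits_PC is a player controller for clicking on characters to test hit reception.
; It shows the mouse cursor and turns on collision display at begin play, then turns the display off at end play.
; A left click runs a complex Visibility trace under the cursor and, if it hits a ThirdPersonCharacter, passes the hit result to that actor's HitReceiver component.
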(event EventBeginPlay
  (Variables|Default|SetbShowMouseCursor true)
  (Development|ExecuteConsoleCommand "ShowFlag.Collision 1" self))

(event EventEndPlay
  (params (EndPlayReason :type EEndPlayReason%20Enum :default "Destroyed"))
  (Development|ExecuteConsoleCommand "ShowFlag.Collision 0" self))

(event Input|MouseEvents|LeftMouseButton
  (params (Key :type Key%20Structure :default "None"))
  (bind (_hitresult _returnvalue) (Game|Player|GetHitResultUnderCursorbyChannel "TraceTypeQuery1" true))
  (:Pressed
    (if _returnvalue
      (bind _asthird_person_character (Utilities|Casting|CastToThirdPersonCharacter (.HitActor (Collision|BreakHitResult _hitresult))))
      (Class|HitReceiver|ReceiveHit (Actor|GetComponentbyClass _asthird_person_character "/Script/Hits.HitReceiver") _hitresult))))

(fn ConstructionScript)